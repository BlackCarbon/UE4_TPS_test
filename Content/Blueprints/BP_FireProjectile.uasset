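; Fire projectile for a team-based TPS that explodes on impact, dealing area damage and destroying itself.
; Hit handling is gated on authority, then builds an ignore set of the owner's teammates, found through TPSGameState, plus all StoneBase actors.
; The explosion applies random, full radial damage to everything else in radius, including potentially the owner, and spawns a shockwave emitter.
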(event Custom|TPS_FireHit
  (params (hit :type Hit%20Result%20Structure))
  ;[1 1 1] Hit event
  (CallFunction|Ignor)
  (CallFunction|Explore (.Location (Collision|BreakHitResult hit))))

(event Custom|ignor
  ;[1 1 1] Hit event
  (Utilities|FlowControl|Sequence
    (:then_0
      (bind _outactors (Actor|GetAllActorsOfClass "/Script/TPS.TPSCharacter"))
      (for _array_element _outactors
        (bind _as角色 (Utilities|Casting|CastToCharacter _array_element))
        (CallFunction|IsFriend _as角色)
        (if (Variables|Default|Getis%20friend)
          (bind _output_get (Variables|Default|Setcharacter _as角色))
          (Utilities|Set|Add (Variables|Default|Getacotor) _output_get))))
    (:then_1
      (bind _outactors_2 (Actor|GetAllActorsOfClass "/Script/TPS.StoneBase"))
      (for _array_element_2 _outactors_2
        (Utilities|Set|Add (Variables|Default|Getacotor) _array_element_2)))))

(event Custom|Fire%20Effect
  (params (Location :type Vector))
  ;[1 1 1] Fire Event
  (Effects|SpawnEmitteratLocation "/Game/FXVarietyPack/Particles/P_ky_shotShockwave.P_ky_shotShockwave" Location))

(event Custom|Explore
  (params (Origin :type Vector%20%28by%20ref%29))
  ;[1 1 1] Hit event
  (bind _result (Utilities|Set|ToArray (Variables|Default|Getacotor)))
  ;;[1 1 1] 造成伤害r
  (Game|Damage|ApplyRadialDamage (Math|Random|RandomFloatinRangefromStream 1e+01 15.0 (Variables|Default|Getrandom%20string)) Origin (Variables|Default|GetDamage%20Radius) 0 _result self (Game|GetInstigatorController (Components|GetOwner)) true "ECC_Visibility")
  (CallFunction|FireEffect Origin))

(event Custom|IsFriend
  (params (player :type Actor%20Object%20Reference))
  ;[1 1 1] IS Friend？
  (bind _astpsgame_state (Utilities|Casting|CastToTPSGameState (Game|GetGameState)))
  (bind _returnvalue (Class|TPSGameState|GetTeamStatebyActor _astpsgame_state (Components|GetOwner self)))
  (bind _returnvalue_2 (Class|TPSGameState|GetTeamStatebyActor _astpsgame_state player))
  (if (== _returnvalue_2 _returnvalue)
    (if (!= (Components|GetOwner self) player)
      (Variables|Default|Setis%20friend true)
      (else
        (Variables|Default|Setis%20friend false)))
    (else
      (Variables|Default|Setis%20friend false))))

(event Collision|EventHit
  (params (MyComp :type Primitive%20Component%20Object%20Reference) (Other :type Actor%20Object%20Reference) (OtherComp :type Primitive%20Component%20Object%20Reference) (bSelfMoved :type Boolean) (HitLocation :type Vector :default "0, 0, 0") (HitNormal :type Vector :default "0, 0, 0") (NormalImpulse :type Vector :default "0, 0, 0") (Hit :type Hit%20Result%20Structure%20%28by%20ref%29))
  ;[1 1 1] 联网
  (Networking|SwitchHasAuthority
    (:Authority
      (CallFunction|TPSFireHit Hit)
      (Actor|DestroyActor self))))

(fn ConstructionScript)