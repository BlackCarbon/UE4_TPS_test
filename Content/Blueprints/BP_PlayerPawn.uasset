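; Player pawn for a team-based third-person shooter, handling the weapon, team visuals and ammo.
; BeginPlay attaches a BP_Gun, then after a delay reads the controller's team from TPSGameState to choose water or fire projectiles, crosshair widget and attached blue or red team light.
; Looping timers poll Died to expire the light.
; Left click fires and spends ammo; R or an empty magazine triggers a montage-and-delay reload from reserve bullets.
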(event Custom|TPS_Fire
  ;[1 1 1] Fire function
  (if (Variables|Default|Getcan%20fire)
    (Class|SWeapon|Fire (Variables|Default|GetCurrentWeapon))
    (Variables|Default|Setcan%20fire false)
    (Utilities|FlowControl|Delay (Variables|Default|Getfire%20speed))
    (Variables|Default|Setcan%20fire true)))

(event Custom|reloadbullet
  ;[1 1 1] Reload bullet
  (Animation|Montage|PlayMontage (Variables|Character|GetMesh) "/Game/AnimStarterPack/TPS_Reload.TPS_Reload" 1.0 0.0 "reload"
    (:then
      _)
    (:OnCompleted
      _))
  (Utilities|FlowControl|Delay 2.17)
  (if (>= (+ (Variables|Default|Getbullet) (Variables|Default|GetNumber%20of%20bullets)) 50)
    (Variables|Default|SetNumber%20of%20bullets (- (Variables|Default|GetNumber%20of%20bullets) (- 50 (Variables|Default|Getbullet))))
    (Variables|Default|Setbullet 50)
    (Variables|Default|Setcan%20reload true)
    (else
      (Variables|Default|SetNumber%20of%20bullets 0)
      (Variables|Default|Setbullet (+ (Variables|Default|GetNumber%20of%20bullets) (Variables|Default|Getbullet)))
      (Variables|Default|Setcan%20reload true))))

(event Custom|TPS%20Reload
  ;[1 1 1] Reload bullet
  (if (Variables|Default|Getcan%20reload)
    (Variables|Default|Setcan%20reload false)
    (CallFunction|Reloadbullet)))

(event Custom|角色死亡
  (bind _bluelight (Variables|Default|GetBlueLight))
  (if (Variables|Default|GetbDied)
    (Utilities|IsValid _bluelight
      (:Is%20Valid
        (Actor|SetLifeSpan _bluelight 4.0)))))

(event Custom|fire%20effect
  (bind _returnvalue (Game|SpawnActorfromClass "/Game/Blueprints/BP_BlueTeamLight.BP_BlueTeamLight_C" (Math|Transform|MakeTransform "0, 0,20.000000" "0, 0, 0" "0.600000,0.600000,0.200000") "AlwaysSpawn" 0 0))
  (Variables|Default|SetBlueLight _returnvalue)
  (Transformation|AttachComponentToComponent _returnvalue (Variables|Character|GetMesh) "TeamScoket" "KeepRelative" "SnapToTarget" "KeepRelative" true)
  (Utilities|Time|SetTimerbyEvent (delegate Custom|角色死亡) 3.0 true))

(event Custom|角色死亡1
  (bind _redlight (Variables|Default|GetRedLight))
  (if (Variables|Default|GetbDied)
    (Utilities|IsValid _redlight
      (:Is%20Valid
        (Actor|SetLifeSpan _redlight 4.0)))))

(event Custom|water%20effect
  (bind _returnvalue (Game|SpawnActorfromClass "/Game/Blueprints/BP_RedTeamLight.BP_RedTeamLight_C" (Math|Transform|MakeTransform "0, 0,20.000000" "0, 0, 0" "0.600000,0.600000,0.200000") "AlwaysSpawn" 0 0))
  (Variables|Default|SetRedLight _returnvalue)
  (Transformation|AttachComponentToComponent _returnvalue (Variables|Character|GetMesh) "TeamScoket" "KeepRelative" "SnapToTarget" "KeepRelative" true)
  (Utilities|Time|SetTimerbyEvent (delegate Custom|角色死亡1) 3.0 true))

(event EventBeginPlay
  (bind _returnvalue (Game|GetGameState))
  ;[1 1 1] UI display
  (bind _returnvalue_2 (Game|SpawnActorfromClass "/Game/Blueprints/BP_Gun.BP_Gun_C" (Math|Transform|MakeTransform "-22.000000,6.000000,-10.000000" "0, 0, 0" "3.000000,3.000000,3.000000") "AlwaysSpawn" self (Variables|Default|GetInstigator)))
  (Variables|Default|SetCurrentWeapon _returnvalue_2)
  (Transformation|AttachComponentToComponent _returnvalue_2 (Variables|Character|GetMesh) "WeaponSkt" "KeepRelative" "SnapToTarget" "KeepRelative" true)
  (Utilities|FlowControl|Delay 5.0)
  (Utilities|IsValid _returnvalue
    (:Is%20Valid
      (bind _astpsgame_state (Utilities|Casting|CastToTPSGameState _returnvalue))
      (bind _returnvalue_3 (Class|TPSGameState|GetTeamStatebyController _astpsgame_state (Pawn|GetController self)))
      (if (!= _returnvalue_3 0)
        (Variables|/Script/TPS.SWeapon|SetProjectileClass _returnvalue_2 "/Game/Blueprints/BP_WaterProjectile.BP_WaterProjectile_C")
        (Development|PrintString "hello")
        (bind _returnvalue_4 (UserInterface|CreateWidget "/Game/Blueprints/UI/BP_BCross.BP_BCross_C"))
        (Utilities|IsValid _returnvalue_4
          (:Is%20Valid
            (UserInterface|Viewport|AddtoViewport _returnvalue_4 0)
            (CallFunction|FireEffect)))
        (else
          (Variables|/Script/TPS.SWeapon|SetProjectileClass _returnvalue_2 "/Game/Blueprints/BP_FireProjectile.BP_FireProjectile_C")
          (Development|PrintString "1")
          (bind _returnvalue_5 (UserInterface|CreateWidget "/Game/Blueprints/UI/BP_RCross.BP_RCross_C"))
          (Utilities|IsValid _returnvalue_5
            (:Is%20Valid
              (UserInterface|Viewport|AddtoViewport _returnvalue_5 0)
              (CallFunction|WaterEffect))))))))

(event Input|KeyboardEvents|R
  (params (Key :type Key%20Structure :default "None"))
  ;[1 1 1] Reload bullet
  (:Pressed
    (CallFunction|TPSReload)))

(event Input|MouseEvents|LeftMouseButton
  (params (Key :type Key%20Structure :default "None"))
  (bind _currentweapon (Variables|Default|GetCurrentWeapon))
  (:Pressed
    (if (Variables|Default|Getcan%20reload)
      ;[1 1 1] Fire function
      (Utilities|IsValid _currentweapon
        (:Is%20Valid
          (Class|SWeapon|Fire _currentweapon)
          (if (!= (Variables|Default|Getbullet) 0)
            (if (!= (Variables|Default|Getbullet) 0)
              (Math|Integer|DecrementInt (Variables|Default|Getbullet)
                (:%20%20
                  (CallFunction|TPSFire)
                  (Audio|PlaySound2D "/Game/FXVarietyPack/Sounds/SW_GunFire.SW_GunFire" 1.0 1.0 0.0 0 0))))
            (elif (>= (Variables|Default|GetNumber%20of%20bullets) 1)
              (CallFunction|TPSReload))))))))

(fn ConstructionScript)