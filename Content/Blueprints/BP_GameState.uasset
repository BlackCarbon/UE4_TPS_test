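; BP_GameState manages which full-game status widget is on screen as the match moves through preparing, in-game and finished phases.
; The GetWidget event switches on the new status to create the matching UI widget and add it to the viewport.
; The In Game and Game Finished phases first remove the preceding phase's widget, and show their own only if that earlier widget is valid, so transitions depend on running in order.
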(event EventGetWidget
  (params (NewStatus :type EGameStatus%20Enum :default "Idle") (OldStatus :type EGameStatus%20Enum :default "Idle"))
  (switch Utilities|FlowControl|Switch|SwitchonEGameStatus NewStatus
    (:PreparingGame
      (bind _returnvalue (UserInterface|CreateWidget "/Game/Blueprints/UI/BP_UI_GamePreparing.BP_UI_GamePreparing_C"))
      (UserInterface|Viewport|AddtoViewport _returnvalue 0))
    (:InGame
      (Utilities|IsValid _returnvalue
        (:Is%20Valid
          (Widget|RemovefromParent _returnvalue)
          (bind _returnvalue_2 (UserInterface|CreateWidget "/Game/Blueprints/UI/BP_UI_InGame.BP_UI_InGame_C"))
          (UserInterface|Viewport|AddtoViewport _returnvalue_2 0))))
    (:GameFinished
      (Utilities|IsValid _returnvalue_2
        (:Is%20Valid
          (Widget|RemovefromParent _returnvalue_2)
          (bind _returnvalue_3 (UserInterface|CreateWidget "/Game/Blueprints/UI/BP_UI_FinshGame.BP_UI_FinshGame_C"))
          (UserInterface|Viewport|AddtoViewport _returnvalue_3 0))))))

(fn ConstructionScript)