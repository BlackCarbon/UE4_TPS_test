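; Water projectile that explodes on hit, dealing random full radial damage and spawning a water-ball impact particle.
; Hit handling runs only with authority: it triggers the explosion, then destroys the projectile.
; Before damage is applied, it builds an ignore set of all StoneBase actors and the owner's teammates, found via TPSGameState team lookups.
; The owner itself is not added to that ignore set.
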(event Custom|TPS%20fire_effect
  (params (Location :type Vector))
  ;[1 1 1] Fire effect
  (Effects|SpawnEmitteratLocation "/Game/FXVarietyPack/Particles/P_ky_waterBallHit.P_ky_waterBallHit" Location))

(event Custom|TPS_waterHit
  (params (Hit :type Hit%20Result%20Structure%20%28by%20ref%29))
  (CallFunction|Ignor)
  (CallFunction|Explore (.Location (Collision|BreakHitResult Hit))))

(event Custom|ignor
  (Utilities|FlowControl|Sequence
    (:then_0
      (bind _outactors (Actor|GetAllActorsOfClass "/Script/TPS.TPSCharacter"))
      (for _array_element _outactors
        (bind _as角色 (Utilities|Casting|CastToCharacter _array_element))
        (CallFunction|IsFriend _as角色)
        (if (Variables|Default|Getis%20friends)
          (bind _output_get (Variables|Default|SetFriend _as角色))
          (Utilities|Set|Add (Variables|Default|Getdont%20damage%20actor) _output_get))))
    (:then_1
      (bind _outactors_2 (Actor|GetAllActorsOfClass "/Script/TPS.StoneBase"))
      (for _array_element_2 _outactors_2
        (Utilities|Set|Add (Variables|Default|Getdont%20damage%20actor) _array_element_2)))))

(event Custom|IsFriend
  (params (player :type Actor%20Object%20Reference))
  ;[1 1 1] IS Friend?
  (bind _astpsgame_state (Utilities|Casting|CastToTPSGameState (Game|GetGameState)))
  (bind _returnvalue (Class|TPSGameState|GetTeamStatebyActor _astpsgame_state (Components|GetOwner self)))
  (bind _returnvalue_2 (Class|TPSGameState|GetTeamStatebyActor _astpsgame_state player))
  (if (== _returnvalue_2 _returnvalue)
    (if (!= (Components|GetOwner self) player)
      (Variables|Default|Setis%20friends true)
      (else
        (Variables|Default|Setis%20friends false)))
    (else
      (Variables|Default|Setis%20friends false))))

(event Custom|Explore
  (params (Origin :type Vector%20%28by%20ref%29))
  (bind _result (Utilities|Set|ToArray (Variables|Default|Getdont%20damage%20actor)))
  ;[1 1 1] 如果撞击的对象是character
  (Game|Damage|ApplyRadialDamage (Math|Random|RandomFloatinRangefromStream 1e+01 15.0 (Variables|Default|GetRandom%20Dange%20String)) Origin (Variables|Default|GetDamage%20radius) 0 _result self (Game|GetInstigatorController (Components|GetOwner)) true "ECC_Visibility")
  (CallFunction|TPSFireEffect Origin))

(event Collision|EventHit
  (params (MyComp :type Primitive%20Component%20Object%20Reference) (Other :type Actor%20Object%20Reference) (OtherComp :type Primitive%20Component%20Object%20Reference) (bSelfMoved :type Boolean) (HitLocation :type Vector :default "0, 0, 0") (HitNormal :type Vector :default "0, 0, 0") (NormalImpulse :type Vector :default "0, 0, 0") (Hit :type Hit%20Result%20Structure%20%28by%20ref%29))
  ;[1 1 1] 联网
  (Networking|SwitchHasAuthority
    (:Authority
      (CallFunction|TPSWaterHit Hit)
      (Actor|DestroyActor self))))

(fn ConstructionScript)