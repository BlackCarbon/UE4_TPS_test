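; Team capture flag that water and fire teams claim, shown by an elemental ball emitter rising along the flag.
; WaterFlag and FireFlag toggle two looping timers; the water tick moves Height by a settable speed, setting owner and spawning a circle effect at the top, clearing at zero.
; Fire's matching movement logic and the overlap-based controller tracking are disconnected, so fire only spawns its emitter and the dead-character cleanup does nothing.
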(event OnComponentBeginOverlap(flag)
  (params (OverlappedComponent :type Primitive%20Component%20Object%20Reference) (OtherActor :type Actor%20Object%20Reference) (OtherComp :type Primitive%20Component%20Object%20Reference) (OtherBodyIndex :type Integer) (bFromSweep :type Boolean) (SweepResult :type Hit%20Result%20Structure%20%28by%20ref%29))
  ;[1 1 1] 查询人数
)

(event OnComponentEndOverlap(Box)
  (params (OverlappedComponent :type Primitive%20Component%20Object%20Reference) (OtherActor :type Actor%20Object%20Reference) (OtherComp :type Primitive%20Component%20Object%20Reference) (OtherBodyIndex :type Integer))
  ;[1 1 1] 查询人数
)

(event Custom|water%20team%20flag
  (bind _flag (Variables|Default|Getflag))
  (bind _water_emitter (Variables|组件|Getwater%20emitter))
  ;[1 1 1] 旗子的上升与下降
  ;;[1 1 1] water
  (CallFunction|GenerateWaterFlag)
  (Utilities|IsValid (Variables|组件|Getwater%20emitter)
    (:Is%20Valid
      (Variables|Default|Setheight%20 (+ (Variables|Default|Getheight%20) (Variables|Default|Getwater%20speed)))
      (Transformation|SetWorldLocation (Variables|组件|Getwater%20emitter) (+ (Transformation|GetWorldLocation _flag) (* (Math|Vector|GetUpVector (Transformation|GetWorldRotation _flag)) (Math|Float|Truncate (/ (Variables|Default|Getheight%20) 4.0)))) false false)
      (if (<= (Variables|Default|Getheight%20) 0.0)
        ;;[1 1 1] water占领被结束
        (Variables|Default|Setwater%20complete false)
        (Utilities|FlowControl|Sequence
          (:then_0
            (Utilities|IsValid _water_emitter
              (:Is%20Valid
                (Components|DestroyComponent _water_emitter)
                (Variables|Default|Setwater%20complete false)
                (Variables|Default|Setflagteam 0))))
          (:then_1
            (Utilities|IsValid (Variables|组件|Getwater%20circle)
              (:Is%20Valid
                (Components|DestroyComponent (Variables|组件|Getwater%20circle))))))
        (else
          ;;[1 1 1] water 完成占领
          (if (>= (Variables|Default|Getheight%20) 3e+03)
            (if (not (Variables|Default|Getwater%20complete))
              (bind _returnvalue (Effects|SpawnEmitteratLocation "/Game/FXVarietyPack/Particles/flag_water.flag_water" (Transformation|GetWorldLocation (Variables|Default|Getflag)) "0, 0, 0" "2.000000,2.000000,2.000000" false))
              (Variables|组件|Setwater%20circle _returnvalue)
              (Variables|Default|Setwater%20complete true)
              (bind _output_get (Variables|Default|Setflagteam 1))
              (Development|PrintString (Utilities|String|ToString(Integer) _output_get)))))))))

(event Custom|Remove%20Died%20Character
  ;[1 1 1] 旗子的上升与下降
  (for _array_element (Variables|Default|Getflagcontroller)
    (Utilities|Casting|CastToPlayerController _array_element)))

(event Custom|generate%20fire%20flag
  ;[1 1 1] 生成旗帜
  (Utilities|IsValid (Variables|组件|Getfire%20emitter)
    (:Is%20Not%20Valid
      (Utilities|IsValid (Variables|组件|Getwater%20emitter)
        (:Is%20Not%20Valid
          (bind _returnvalue (Effects|SpawnEmitteratLocation "/Game/FXVarietyPack/Particles/P_ky_fireBall.P_ky_fireBall" (Transformation|GetWorldLocation (Variables|Default|Getflag)) "0, 0, 0" "1.000000,1.000000,1.000000" false))
          (Variables|组件|Setfire%20emitter _returnvalue))))))

(event Custom|generate%20water%20flag
  ;[1 1 1] 生成旗帜
  (Utilities|IsValid (Variables|组件|Getfire%20emitter)
    (:Is%20Not%20Valid
      (Utilities|IsValid (Variables|组件|Getwater%20emitter)
        (:Is%20Not%20Valid
          (bind _returnvalue (Effects|SpawnEmitteratLocation "/Game/FXVarietyPack/Particles/P_ky_waterBall.P_ky_waterBall" (Transformation|GetWorldLocation (Variables|Default|Getflag)) "0, 0, 0" "1.000000,1.000000,1.000000" false))
          (Variables|组件|Setwater%20emitter _returnvalue))))))

(event Custom|fire%20team%20flag
  ;[1 1 1] 旗子的上升与下降
  ;;[1 1 1] Fire
  (CallFunction|GenerateFireFlag)
  (Utilities|IsValid (Variables|组件|Getfire%20emitter)))

(event EventSetSpeed
  (params (speed :type Float%20%28single-precision%29))
  (Utilities|FlowControl|Sequence
    (:then_0
      (Variables|Default|Setfirespeed speed))
    (:then_1
      (Variables|Default|Setwater%20speed speed))))

(event EventFireFlag
  (Utilities|Time|PauseTimerbyHandle (Variables|Default|Getwatertime))
  (Utilities|Time|UnpauseTimerbyHandle (Variables|Default|Getfiretime)))

(event EventSetColor
  (Utilities|IsValid (Variables|组件|Getwater%20emitter)
    (:Is%20Valid
      (Variables|Default|Setflagcolor 2))
    (:Is%20Not%20Valid
      (Utilities|IsValid (Variables|组件|Getfire%20emitter)
        (:Is%20Valid
          (Variables|Default|Setflagcolor 1))
        (:Is%20Not%20Valid
          (Variables|Default|Setflagcolor 0))))))

(event EventBeginPlay
  (Utilities|FlowControl|Sequence
    (:then_0
      (bind _returnvalue (Utilities|Time|SetTimerbyEvent (delegate Custom|water%20team%20flag) 0.001 true))
      ;[1 1 1] 旗子的上升与下降
      (bind _output_get (Variables|Default|Setwatertime _returnvalue))
      (Utilities|Time|PauseTimerbyHandle _output_get))
    (:then_1
      (bind _returnvalue_2 (Utilities|Time|SetTimerbyEvent (delegate Custom|fire%20team%20flag) 0.001 true))
      (bind _output_get_2 (Variables|Default|Setfiretime _returnvalue_2))
      (Utilities|Time|PauseTimerbyHandle _output_get_2))
    (:then_2
      (Utilities|Time|SetTimerbyEvent (delegate Custom|Remove%20Died%20Character) 0.001 true))))

(event EventWaterFlag
  (Utilities|Time|PauseTimerbyHandle (Variables|Default|Getfiretime))
  (Utilities|Time|UnpauseTimerbyHandle (Variables|Default|Getwatertime)))

(fn ConstructionScript)